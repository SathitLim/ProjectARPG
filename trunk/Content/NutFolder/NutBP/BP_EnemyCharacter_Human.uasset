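; Human enemy character Blueprint with events for chasing the player, range-checked attacks and stagger.
; AI MoveTo handles pursuit or forced moves, and a timeline interpolates rotation toward the player.
; Distance bands all lead to StartAttack, which picks a random attack index; cooldown and DoOnce flags gate attacks and stagger.
; The looping seek and distance timers are disconnected, so BeginPlay only delays.
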(event `self.ReceiveBeginPlay`
  (`KismetSystemLibrary.Delay` 0.2))

(event `SeekPlayer`
  (`|AIMoveTo` self (0.0 0.0 0.0) (`GameplayStatics.GetPlayerCharacter` 0) 200.0))

(event `ForceMoveto`
  (params (Location :type "Vector Structure" :default (0.0 0.0 0.0)))
  (`|AIMoveTo` self Location null 200.0))

(event `DistancePlayer`
  (if (not (`self.IsAttack?`))
    (bind _output_get (set `self.Distance` (`KismetMathLibrary.VSize` (- (`self.K2_GetActorLocation`) (`self.K2_GetActorLocation` (`GameplayStatics.GetPlayerCharacter` 0))))))
    (if (<= _output_get 200.0)
      (`KismetSystemLibrary.PrintString` "Atk1")
      (`self.StartAttack` :!label _label)
      (elif (<= _output_get 300.0)
        (`KismetSystemLibrary.PrintString` "Atk2")
        (goto _label)
        (elif (<= _output_get 400.0)
          (`KismetSystemLibrary.PrintString` "Atk3")
          (goto _label))))))

(event `FacePlayer`
  (`Timeline|FaceToPlayer` :!via `PlayFromStart`
    (:`Update`
      (`self.K2_SetActorRotation` (`KismetMathLibrary.RInterpTo` (`self.K2_GetActorRotation`) (`KismetMathLibrary.FindLookAtRotation` (`self.K2_GetActorLocation`) (`self.K2_GetActorLocation` (`GameplayStatics.GetPlayerCharacter` 0))) 1.0 0.1)))))

(event `StartAttack`
  (if (`self.CanAttack`)
    (set `self.IsAttack?` true)
    (set `self.numAtk` (`KismetMathLibrary.RandomInteger` 5))))

(event `EndAttack`
  (set `self.IsAttack?` false)
  (set `self.CanAttack` false)
  (`KismetSystemLibrary.Delay` 1.0)
  (set `self.CanAttack` true))

(event `StartStugger`
  (`/Engine/EditorBlueprintResources/StandardMacros.DoOnce` false :!label _label_2
    (:`Completed`
      (set `self.IsStugger?` true))))

(event `EndStugger`
  (set `self.IsStugger?` false)
  (`KismetSystemLibrary.Delay` 0.5)
  (goto _label_2 :!via `Reset`))

(event `self.CapsuleComponent.OnComponentBeginOverlap`
  (params (OverlappedComponent :type "PrimitiveComponent Object Reference") (OtherActor :type "Actor Object Reference") (OtherComp :type "PrimitiveComponent Object Reference") (OtherBodyIndex :type Integer) (bFromSweep :type Boolean) (SweepResult :type "HitResult Structure (by ref)")))

(fn `UserConstructionScript`
  (`parent.UserConstructionScript`))